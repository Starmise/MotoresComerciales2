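; Behavior tree task that walks the controlled pawn around the patrol path stored on its AI_BehaviourComponent, failing if the component or path is missing.
; The path's map keys are waypoint actors visited in order, each followed by a timer using that entry's WaitTime.
; The index wraps to loop indefinitely, so the task never finishes successfully and ends itself only on failure, including failed moves.
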(event `self.ReceiveExecuteAI`
  (params (OwnerController :type "AIController Object Reference") (ControlledPawn :type "Pawn Object Reference"))
  (bind _returnvalue (`Actor.GetComponentByClass` ControlledPawn "/Game/AI/Blueprints/AI_BehaviourComponent.AI_BehaviourComponent_C"))
  (bind _patrolpath (`/Game/AI/Blueprints/AI_BehaviourComponent.PatrolPath` _returnvalue))
  (bind _returnvalue_2 (`BlueprintMapLibrary.Map_Length` _patrolpath))
  (set `self.Controlled Pawn` ControlledPawn)
  (`/Engine/EditorBlueprintResources/StandardMacros.IsValid` _returnvalue
    (:`Is Valid`
      (`KismetSystemLibrary.PrintString` (`KismetStringLibrary.Conv_IntToString` _returnvalue_2))
      (if (> _returnvalue_2 0)
        (set `self.Patrol Path` _patrolpath)
        (`self.MoveToPatrolPath`)
        (else
          (`self.FinishExecute` false))))
    (:`Is Not Valid`
      (`self.FinishExecute` false))))

(event `MoveToPatrolPath`
  (bind _keys (`BlueprintMapLibrary.Map_Keys` (`self.Patrol Path`)))
  (`|AIMoveTo` (`self.Controlled Pawn`) (`Actor.K2_GetActorLocation` (`|GetArrayItem` _keys (`self.CurrentPatrolID`))) null
    (:`OnSuccess`
      (bind _keys_2 (`BlueprintMapLibrary.Map_Keys` (`self.Patrol Path`)))
      (`KismetSystemLibrary.K2_SetTimerDelegate` (delegate `OnEndWait`) (`KismetMathLibrary.FMax` (break `/Game/AI/Blueprints/Struct_PatrolPath` (`BlueprintMapLibrary.Map_Find` (`self.Patrol Path`) (`|GetArrayItem` _keys_2 (`self.CurrentPatrolID`)))) 0.1)))
    (:`OnFail`
      (`KismetSystemLibrary.PrintString` "No Move To")
      (`self.FinishExecute` false))))

(event `OnEndWait`
  (bind _result (`/Engine/EditorBlueprintResources/StandardMacros.IncrementInt` (`self.CurrentPatrolID`))
    (:`  `
      (if (>= _result (`BlueprintMapLibrary.Map_Length` (`self.Patrol Path`)))
        (set `self.CurrentPatrolID` 0)
        (`self.MoveToPatrolPath`)
        (else
          (`self.MoveToPatrolPath`))))))