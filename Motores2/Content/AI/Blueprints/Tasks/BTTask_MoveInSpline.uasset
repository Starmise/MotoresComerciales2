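; Behavior tree task that toggles movement on a BP_PerceptionNPC_Spline pawn, by its name for movement along a spline.
; On execute it casts and caches the controlled pawn.
; Each tick it copies the CanMoveKey blackboard bool into the pawn's CanMove flag, leaving the movement itself to the pawn.
; It never calls Finish Execute, so it keeps running until interrupted.
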(event `self.ReceiveExecuteAI`
  (params (OwnerController :type "AIController Object Reference") (ControlledPawn :type "Pawn Object Reference"))
  (bind _asbp_perception_npc_spline (cast `/Game/AI/Blueprints/BP_PerceptionNPC_Spline` ControlledPawn))
  (set `self.npcPawn` _asbp_perception_npc_spline))

(event `self.ReceiveTickAI`
  (params (OwnerController :type "AIController Object Reference") (ControlledPawn :type "Pawn Object Reference") (DeltaSeconds :type "Float (single-precision)"))
  (bind _npcpawn (`self.npcPawn`))
  (if (`KismetSystemLibrary.IsValid` (`self.npcPawn`))
    (if (`BlackboardComponent.GetValueAsBool` (`AIBlueprintHelperLibrary.GetBlackboard` OwnerController) (`self.canMoveKey`))
      (set `/Game/AI/Blueprints/BP_PerceptionNPC_Spline.canMove` true _npcpawn)
      (else
        (set `/Game/AI/Blueprints/BP_PerceptionNPC_Spline.canMove` false _npcpawn)))))