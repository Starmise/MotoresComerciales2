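; BP_FloorBlend is a floor actor that gradually shifts its snow-blend material during play, apparently to show snow accumulating.
; The construction script creates a dynamic instance of M_BlendSnow on the Cube component.
; On BeginPlay, a looping timer repeatedly calls MatAccomulation, which nudges the material's "Bias (S)" scalar upward in small steps.
; A delay then clears the timer, so the buildup stops after a fixed period.
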(event `self.ReceiveBeginPlay`
  (bind _returnvalue (`KismetSystemLibrary.K2_SetTimer` null "MatAccomulation" 0.3 true))
  (`KismetSystemLibrary.Delay` 20.0)
  (`KismetSystemLibrary.K2_ClearAndInvalidateTimerHandle` _returnvalue))

(fn `MatAccomulation`
  (bind _matinst (`self.MatInst`))
  (bind _returnvalue (`MaterialInstanceDynamic.K2_GetScalarParameterValue` _matinst "Bias (S)"))
  (`MaterialInstanceDynamic.SetScalarParameterValue` _matinst "Bias (S)" (+ _returnvalue 0.04)))

(fn `UserConstructionScript`
  (bind _returnvalue (`PrimitiveComponent.CreateDynamicMaterialInstance` (`self.Cube`) 0 "/Game/MaterialsOG/Snow/M_BlendSnow.M_BlendSnow" "None"))
  (set `self.MatInst` _returnvalue))